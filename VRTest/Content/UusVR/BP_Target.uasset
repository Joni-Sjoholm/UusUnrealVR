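; BP_Target is a VR shooting target that awards score and rotates when something overlaps it.
; Overlapping Box adds 10 to the player VRPawn's Score, while HeadBox adds 25; neither checks the overlapping actor.
; Both then play the TargetRotate timeline, which drives the actor's relative roll.
; Every timeline update also plays a metal bullet-hit sound at the world origin rather than at the target.
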(event `self.Box.OnComponentBeginOverlap`
  (params (OverlappedComponent :type "PrimitiveComponent Object Reference") (OtherActor :type "Actor Object Reference") (OtherComp :type "PrimitiveComponent Object Reference") (OtherBodyIndex :type Integer) (bFromSweep :type Boolean) (SweepResult :type "HitResult Structure (by ref)"))
  (bind _asvrpawn (cast `/Game/UusVR/VRTemplate/Blueprints/VRPawn` (`GameplayStatics.GetPlayerPawn` 0)))
  (set `/Game/UusVR/VRTemplate/Blueprints/VRPawn.Score` (+ (`/Game/UusVR/VRTemplate/Blueprints/VRPawn.Score` _asvrpawn) 10) _asvrpawn)
  (bind (_direction _targetrotvalue) (`Timeline|TargetRotate` :!label _label)
    (:`Update`
      (`self.K2_SetActorRelativeRotation` (`KismetMathLibrary.MakeRotator` _targetrotvalue))
      (`GameplayStatics.PlaySoundAtLocation` "/Game/UusVR/Bullet_Metal_Hit_Sound_Effect__shorts.Bullet_Metal_Hit_Sound_Effect__shorts" (0.0 0.0 0.0) (struct) 1.0 1.0 0.0 null null null null))))

(event `self.HeadBox.OnComponentBeginOverlap`
  (params (OverlappedComponent :type "PrimitiveComponent Object Reference") (OtherActor :type "Actor Object Reference") (OtherComp :type "PrimitiveComponent Object Reference") (OtherBodyIndex :type Integer) (bFromSweep :type Boolean) (SweepResult :type "HitResult Structure (by ref)"))
  (bind _asvrpawn (cast `/Game/UusVR/VRTemplate/Blueprints/VRPawn` (`GameplayStatics.GetPlayerPawn` 0)))
  (set `/Game/UusVR/VRTemplate/Blueprints/VRPawn.Score` (+ (`/Game/UusVR/VRTemplate/Blueprints/VRPawn.Score` _asvrpawn) 25) _asvrpawn)
  (goto _label))

(fn `UserConstructionScript`)